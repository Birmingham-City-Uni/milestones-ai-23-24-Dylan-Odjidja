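; Combat component for the third-person player character that runs a four-step sword and kick melee combo.
; Attack input starts the chain, or buffers the next hit in SaveAttack if an attack is already running.
; SwordAttackCombo consumes that buffer to play the montage selected by AttackIndex, otherwise StopCombo resets the chain.
; Each step uses a DoOnce and short delay before playing its montage on the owner's mesh.
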(event Custom|SwordAttack
  ;[0.05098 0.05098 0.05098] Sword Attack
  (if (Variables|Default|GetIsAttacking)
    (Variables|Default|SetSaveAttack true)
    (else
      (Variables|Default|SetIsAttacking true)
      (switch int (Variables|Default|GetAttack%20Index)
        (:0
          (CallFunction|Attack1))
        (:1
          (CallFunction|Attack2))
        (:2
          (CallFunction|Attack3))
        (:3
          (CallFunction|Attack4))))))

(event Custom|SwordAttackCombo
  ;[0.05098 0.05098 0.05098] Combo
  (if (Variables|Default|GetSaveAttack)
    (Variables|Default|SetSaveAttack false)
    (switch int (Variables|Default|GetAttack%20Index)
      (:0
        (CallFunction|Attack1))
      (:1
        (CallFunction|Attack2))
      (:2
        (CallFunction|Attack3))
      (:3
        (CallFunction|Attack4)))
    (else
      (CallFunction|StopCombo))))

(event Custom|Attack%201
  ;[0.05098 0.05098 0.05098] Attack 1
  (Utilities|FlowControl|DoOnce false :!label _label
    (:Completed
      (Utilities|FlowControl|Delay 0.1)
      (Animation|Montage|PlayMontage (Variables|Default|GetChar%20Mesh) "/Game/Characters/Playable_Character/Animations/Combat/Attack1_Montage.Attack1_Montage"
        (:then
          (Variables|Default|SetAttack%20Index 1)
          (goto _label Reset))))))

(event Custom|Attack%202
  ;[0.05098 0.05098 0.05098] Attack 2
  (Utilities|FlowControl|DoOnce false :!label _label
    (:Completed
      (Utilities|FlowControl|Delay 0.1)
      (Animation|Montage|PlayMontage (Variables|Default|GetChar%20Mesh) "/Game/Characters/Playable_Character/Animations/Combat/Attack2_Montage.Attack2_Montage"
        (:then
          (Variables|Default|SetAttack%20Index 2)
          (goto _label Reset))))))

(event Custom|Attack%203
  ;[0.05098 0.05098 0.05098] Attack 3
  (Utilities|FlowControl|DoOnce false :!label _label
    (:Completed
      (Utilities|FlowControl|Delay 0.1)
      (Animation|Montage|PlayMontage (Variables|Default|GetChar%20Mesh) "/Game/Characters/Playable_Character/Animations/Combat/Kick_Montage.Kick_Montage"
        (:then
          (Variables|Default|SetAttack%20Index 3)
          (goto _label Reset))))))

(event Custom|Attack%204
  ;[0.05098 0.05098 0.05098] Attack 4
  (Utilities|FlowControl|DoOnce false :!label _label
    (:Completed
      (Utilities|FlowControl|Delay 0.1)
      (Animation|Montage|PlayMontage (Variables|Default|GetChar%20Mesh) "/Game/Characters/Playable_Character/Animations/Combat/Attack3_Montage.Attack3_Montage"
        (:then
          (Variables|Default|SetAttack%20Index 4)
          (goto _label Reset))))))

(event Custom|StopCombo
  ;[0.05098 0.05098 0.05098] Stop Combo/Attack
  (Variables|Default|SetIsAttacking false)
  (Variables|Default|SetAttack%20Index 0))

(event Input|EnhancedActionEvents|EnhancedInputActionIA_Attack
  (params (ActionValue :type Boolean) (ElapsedSeconds :type Float%20%28double-precision%29) (TriggeredSeconds :type Float%20%28double-precision%29) (InputAction :type Input%20Action%20Object%20Reference :default "/Game/ThirdPerson/Input/Actions/IA_Attack.IA_Attack"))
  ;[0.05098 0.05098 0.05098] Attack Input
  (:Started
    (if (Variables|Default|GetCanAttack)
      (CallFunction|SwordAttack))))

(event EventBeginPlay
  ;[0.05098 0.05098 0.05098] Get Character Mesh
  (bind _asbp_third_person_character (Utilities|Casting|CastToBP_ThirdPersonCharacter (Components|GetOwner)))
  (Variables|Default|SetChar%20Mesh (Variables|/Script/Engine.Character|GetMesh _asbp_third_person_character)))