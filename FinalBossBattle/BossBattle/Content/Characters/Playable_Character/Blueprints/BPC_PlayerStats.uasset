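; Player stats component that tracks current and max health and stamina for the third-person character.
; On BeginPlay it waits a tick, caches the owning BP_ThirdPersonCharacter and initializes that character's HUD bars and health text.
; Functions decrease, increase (capped at max) or raise the maximum of each stat, pushing changes straight to the HUD widget.
; The decrease functions return true once the stat is depleted.
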(event EventBeginPlay
  (Utilities|FlowControl|DelayUntilNextTick)
  (bind _asbp_third_person_character (Utilities|Casting|CastToBP_ThirdPersonCharacter (Components|GetOwner)))
  (Variables|Default|SetCharacter%20Reference _asbp_third_person_character)
  (Progress|SetPercent (Variables|/Game/Characters/Playable_Character/HUD/WB_HUD.WB_HUD_C|GetStaminaBar (Variables|/Game/ThirdPerson/Blueprints/BP_ThirdPersonCharacter.BP_ThirdPersonCharacter_C|GetHUD%20Widget (Variables|Default|GetCharacter%20Reference))) (/ (Variables|Stamina|GetCurrent%20Stamina) (Variables|Stamina|GetMax%20Stamina)))
  (Progress|SetPercent (Variables|/Game/Characters/Playable_Character/HUD/WB_HUD.WB_HUD_C|GetHealthBar (Variables|/Game/ThirdPerson/Blueprints/BP_ThirdPersonCharacter.BP_ThirdPersonCharacter_C|GetHUD%20Widget (Variables|Default|GetCharacter%20Reference))) (/ (Variables|Health|GetCurrent%20Health) (Variables|Health|GetMax%20Health)))
  (Rendering|Components|TextRender|SetText (Variables|/Game/Characters/Playable_Character/HUD/WB_HUD.WB_HUD_C|GetHealthText (Variables|/Game/ThirdPerson/Blueprints/BP_ThirdPersonCharacter.BP_ThirdPersonCharacter_C|GetHUD%20Widget (Variables|Default|GetCharacter%20Reference))) (Utilities|Text|ToText(Float) (Variables|Health|GetCurrent%20Health) "HalfToEven")))

(fn DecreaseHealth
  (params (Damage :type Float%20%28double-precision%29))
  (bind _character_reference (Variables|Default|GetCharacter%20Reference))
  (bind _hud_widget (Variables|/Game/ThirdPerson/Blueprints/BP_ThirdPersonCharacter.BP_ThirdPersonCharacter_C|GetHUD%20Widget _character_reference))
  (if (not (<= (Variables|Health|GetCurrent%20Health) 0.0))
    (bind _output_get (Variables|Health|SetCurrent%20Health (- (Variables|Health|GetCurrent%20Health) Damage)))
    (Progress|SetPercent (Variables|/Game/Characters/Playable_Character/HUD/WB_HUD.WB_HUD_C|GetHealthBar _hud_widget) (/ _output_get (Variables|Health|GetMax%20Health)))
    (Rendering|Components|TextRender|SetText (Variables|/Game/Characters/Playable_Character/HUD/WB_HUD.WB_HUD_C|GetHealthText _hud_widget) (Utilities|Text|ToText(Float) (Variables|Health|GetCurrent%20Health) "HalfToEven"))
    (if (<= (Variables|Health|GetCurrent%20Health) 0.0)
      _
      (else
        (return false))))
  (return true))

(fn IncreaseMaxHealth
  (params (Health%20Incremntion :type Float%20%28double-precision%29))
  (bind _character_reference (Variables|Default|GetCharacter%20Reference))
  (bind _hud_widget (Variables|/Game/ThirdPerson/Blueprints/BP_ThirdPersonCharacter.BP_ThirdPersonCharacter_C|GetHUD%20Widget _character_reference))
  (Variables|Health|SetMax%20Health (+ (Variables|Health|GetMax%20Health) Health%20Incremntion))
  (Progress|SetPercent (Variables|/Game/Characters/Playable_Character/HUD/WB_HUD.WB_HUD_C|GetHealthBar _hud_widget) (/ (Variables|Health|GetCurrent%20Health) (Variables|Health|GetMax%20Health)))
  (Rendering|Components|TextRender|SetText (Variables|/Game/Characters/Playable_Character/HUD/WB_HUD.WB_HUD_C|GetHealthText _hud_widget) (Utilities|Text|ToText(Float) (Variables|Health|GetCurrent%20Health) "HalfToEven")))

(fn DecreaseStamina
  (params (Stamina%20Depleted :type Float%20%28double-precision%29))
  (if (not (<= (Variables|Stamina|GetCurrent%20Stamina) 0.0))
    (Variables|Stamina|SetCurrent%20Stamina (- (Variables|Stamina|GetCurrent%20Stamina) Stamina%20Depleted))
    (Progress|SetPercent (Variables|/Game/Characters/Playable_Character/HUD/WB_HUD.WB_HUD_C|GetStaminaBar (Variables|/Game/ThirdPerson/Blueprints/BP_ThirdPersonCharacter.BP_ThirdPersonCharacter_C|GetHUD%20Widget (Variables|Default|GetCharacter%20Reference))) (/ (Variables|Stamina|GetCurrent%20Stamina) (Variables|Stamina|GetMax%20Stamina)))
    (if (<= (Variables|Stamina|GetCurrent%20Stamina) 0.0)
      _
      (else
        (return false))))
  (return true))

(fn IncreaseMaxStamina
  (params (Incoming%20Stamina :type Float%20%28double-precision%29))
  (Variables|Stamina|SetMax%20Stamina (+ (Variables|Stamina|GetMax%20Stamina) Incoming%20Stamina))
  (Progress|SetPercent (Variables|/Game/Characters/Playable_Character/HUD/WB_HUD.WB_HUD_C|GetStaminaBar (Variables|/Game/ThirdPerson/Blueprints/BP_ThirdPersonCharacter.BP_ThirdPersonCharacter_C|GetHUD%20Widget (Variables|Default|GetCharacter%20Reference))) (/ (Variables|Stamina|GetCurrent%20Stamina) (Variables|Stamina|GetMax%20Stamina))))

(fn IncreaseHealth
  (params (Added%20Health :type Float%20%28double-precision%29))
  (bind _character_reference (Variables|Default|GetCharacter%20Reference))
  (bind _hud_widget (Variables|/Game/ThirdPerson/Blueprints/BP_ThirdPersonCharacter.BP_ThirdPersonCharacter_C|GetHUD%20Widget _character_reference))
  (Variables|Health|SetCurrent%20Health (+ (Variables|Health|GetCurrent%20Health) Added%20Health))
  (if (> (Variables|Health|GetCurrent%20Health) (Variables|Health|GetMax%20Health))
    (Variables|Health|SetCurrent%20Health (Variables|Health|GetMax%20Health)))
  (Progress|SetPercent (Variables|/Game/Characters/Playable_Character/HUD/WB_HUD.WB_HUD_C|GetHealthBar _hud_widget) (/ (Variables|Health|GetCurrent%20Health) (Variables|Health|GetMax%20Health)))
  (Rendering|Components|TextRender|SetText (Variables|/Game/Characters/Playable_Character/HUD/WB_HUD.WB_HUD_C|GetHealthText _hud_widget) (Utilities|Text|ToText(Float) (Variables|Health|GetCurrent%20Health) "HalfToEven")))

(fn IncreaseStamina
  (params (Added%20Stamina :type Float%20%28double-precision%29))
  (Variables|Stamina|SetCurrent%20Stamina (+ (Variables|Stamina|GetCurrent%20Stamina) Added%20Stamina))
  (if (> (Variables|Stamina|GetCurrent%20Stamina) (Variables|Stamina|GetMax%20Stamina))
    (Variables|Stamina|SetCurrent%20Stamina (Variables|Stamina|GetMax%20Stamina)))
  (Progress|SetPercent (Variables|/Game/Characters/Playable_Character/HUD/WB_HUD.WB_HUD_C|GetStaminaBar (Variables|/Game/ThirdPerson/Blueprints/BP_ThirdPersonCharacter.BP_ThirdPersonCharacter_C|GetHUD%20Widget (Variables|Default|GetCharacter%20Reference))) (/ (Variables|Stamina|GetCurrent%20Stamina) (Variables|Stamina|GetMax%20Stamina))))